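; BP_MoveUpDown is an actor whose Cube oscillates vertically between zero and an EndPoint height while IsPlay is set.
; Tick shifts the cube's relative Z by a fixed step per frame, independent of delta time, reversing at each limit via the misleadingly named IsMoveRight flag.
; BeginPlay binds to the ThirdPersonCharacter's F-key dispatcher, and functions taking a boolean set IsPlay.
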(event EventBeginPlay
  (bind _asthird_person_character (Utilities|Casting|CastToThirdPersonCharacter (Game|GetPlayerCharacter 0)))
  (EventDispatchers|BindEventtoEventDispatcherFKey _asthird_person_character (EventDispatchers|CreateEvent :!event BPMoveUpDownAutoGenFunc)))

(event EventTick
  (params (DeltaSeconds :type Float%20%28single-precision%29))
  (bind _cube (Variables|Default|GetCube))
  (if (Variables|Default|GetisPlay)
    (if (Variables|Default|GetIsMoveRight)
      (Transformation|AddRelativeLocation _cube "0.000000, 0,5.000000" false false)
      (if (>= (.z (Variables|/Script/Engine.SceneComponent|GetRelativeLocation _cube)) (Variables|Default|GetEndPoint))
        (Variables|Default|SetIsMoveRight false))
      (else
        (Transformation|AddRelativeLocation (Variables|Default|GetCube) "0.000000, 0,-5.000000" false false)
        (if (< (.z (Variables|/Script/Engine.SceneComponent|GetRelativeLocation _cube)) 0.0)
          (Variables|Default|SetIsMoveRight true))))))

(fn ConstructionScript)

(fn BPMoveUpDownAutoGenFunc
  (params (Is%20Pressed :type Boolean))
  (Variables|Default|SetisPlay Is%20Pressed))

(fn Play
  (params (isPlay :type Boolean))
  (Variables|Default|SetisPlay isPlay)
  (return true))